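; Player character Blueprint for a Megaman side-scroller, handling Enhanced Input for moving, jumping and shooting.
; Movement runs along world X only, with UpdateRotation snapping controller yaw to 0 or 180 to face the input direction.
; Each shot press spawns a regular projectile at ShootPos and holds IsShooting true through a retriggerable delay of ShootAnimDuration, so rapid fire extends the shooting state.
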(event `self.ReceiveBeginPlay`
  (`parent.ReceiveBeginPlay`))

(event `EnhancedInput|/Game/Megaman/Assets/Input/Actions/IA_Jump`
  (params (ActionValue :type Boolean) (ElapsedSeconds :type "Float (double-precision)") (TriggeredSeconds :type "Float (double-precision)") (InputAction :type "InputAction Object Reference" :default "/Game/Megaman/Assets/Input/Actions/IA_Jump.IA_Jump"))
  (:`Started`
    (`self.Jump`))
  (:`Canceled`
    (`self.StopJumping` :!label _label))
  (:`Completed`
    (goto _label)))

(event `EnhancedInput|/Game/Megaman/Assets/Input/Actions/IA_Movement`
  (params (ActionValue :type "Float (double-precision)") (ElapsedSeconds :type "Float (double-precision)") (TriggeredSeconds :type "Float (double-precision)") (InputAction :type "InputAction Object Reference" :default "/Game/Megaman/Assets/Input/Actions/IA_Movement.IA_Movement"))
  (:`Triggered`
    (`self.AddMovementInput` (1.0 0.0 0.0) ActionValue)
    (`self.UpdateRotation` ActionValue)))

(event `EnhancedInput|/Game/Megaman/Assets/Input/Actions/IA_Shoot`
  (params (ActionValue :type Boolean) (ElapsedSeconds :type "Float (double-precision)") (TriggeredSeconds :type "Float (double-precision)") (InputAction :type "InputAction Object Reference" :default "/Game/Megaman/Assets/Input/Actions/IA_Shoot.IA_Shoot"))
  (bind _shootpos (`self.ShootPos`))
  (:`Started`
    (set `self.IsShooting` true)
    (`|SpawnActorFromClass` "/Game/Megaman/Assets/Blueprints/Projectiles/Player/BP_PlayerProjectile_RegularShot.BP_PlayerProjectile_RegularShot_C" (`KismetMathLibrary.MakeTransform` (`SceneComponent.K2_GetComponentLocation` _shootpos) (`SceneComponent.K2_GetComponentRotation` _shootpos)) "AlwaysSpawn" "MultiplyWithRoot" self self)
    (`KismetSystemLibrary.RetriggerableDelay` (`self.ShootAnimDuration`))
    (set `self.IsShooting` false)))

(fn `UpdateRotation`
  (params (A :type "Float (double-precision)"))
  (`Controller.SetControlRotation` (`self.GetController`) (select `bool` (>= A 0.0) :`false` (`KismetMathLibrary.MakeRotator` 0.0 0.0 180.0) :`true` (`KismetMathLibrary.MakeRotator` 0.0))))

(fn `UserConstructionScript`
  (`parent.UserConstructionScript`))